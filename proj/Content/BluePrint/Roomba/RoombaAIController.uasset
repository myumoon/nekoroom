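; AI controller for the Roomba that starts its behavior tree when play begins.
; On BeginPlay it sets up the Roomba blackboard, seeds the MovePos key with a hardcoded location, runs the RoombaAI tree and prints whether it started.
; Tick is empty, and a leftover node chain that would nudge the pawn along Y is disconnected and never runs.
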(event EventBeginPlay
  (bind _blackboardcomponent (Class|AIController|UseBlackboard "/Game/BluePrint/Roomba/RoombaBlackboard.RoombaBlackboard"))
  (AI|Components|Blackboard|SetValueasVector _blackboardcomponent (Utilities|String|StringToName (Utilities|String|MakeLiteralString "MovePos")) "-400.000000,0.000000,130.000000")
  (bind _returnvalue (AI|RunBehaviorTree "/Game/BluePrint/Roomba/RoombaAI.RoombaAI"))
  (Development|PrintString (Utilities|String|ToString(Boolean) _returnvalue)))

(event EventTick
  (params (DeltaSeconds :type Float%20%28single-precision%29)))

(fn ConstructionScript)