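; Roomba robot actor that senses obstacles and reports them to its RoombaAIController.
; Its Cylinder overlap, gated by a DoOnce until the overlap ends, sends the hit location as a wall-sensor event and marks forward movement as blocked.
; CheckForwardVolume counts overlapping objects and reports forward movement as possible again when the count returns to zero.
; A forward line trace on Tick only draws debug, as its result is unused.
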(event OnComponentBeginOverlap(Cylinder)
  (params (OtherActor :type Actor%20Object%20Reference) (OtherComp :type Primitive%20Component%20Object%20Reference) (OtherBodyIndex :type Integer) (bFromSweep :type Boolean) (SweepResult :type Hit%20Result%20Structure%20%28by%20ref%29))
  ;[1 1 1] オブジェクトに当たった時の挙動
  (Utilities|FlowControl|DoOnce false
    (:Completed
      (Development|PrintString "Hiiiit")
      (bind _returnvalue (AI|GetAIController self))
      (bind _asroomba_aicontroller (Utilities|Casting|CastToRoombaAIController _returnvalue))
      (Default|NotifyWallSensor _asroomba_aicontroller (.Location (Collision|BreakHitResult SweepResult)))
      (Default|NotifyMovableForward _asroomba_aicontroller false))))

(event OnComponentBeginOverlap(CheckForwardVolume)
  (params (OtherActor :type Actor%20Object%20Reference) (OtherComp :type Primitive%20Component%20Object%20Reference) (OtherBodyIndex :type Integer) (bFromSweep :type Boolean) (SweepResult :type Hit%20Result%20Structure%20%28by%20ref%29))
  ;[1 1 1] 前方に進めるようになった時の挙動ヒットしているオブジェクトが無くなったら進める
  (Variables|Default|SetForwardOverlapObjects (+ (Variables|Default|GetForwardOverlapObjects) 1)))

(event OnComponentEndOverlap(CheckForwardVolume)
  (params (OtherActor :type Actor%20Object%20Reference) (OtherComp :type Primitive%20Component%20Object%20Reference) (OtherBodyIndex :type Integer))
  ;[1 1 1] 前方に進めるようになった時の挙動ヒットしているオブジェクトが無くなったら進める
  (bind _output_get (Variables|Default|SetForwardOverlapObjects (+ (Variables|Default|GetForwardOverlapObjects) -1)))
  (if (== _output_get 0)
    (bind _returnvalue (AI|GetAIController self))
    (bind _asroomba_aicontroller (Utilities|Casting|CastToRoombaAIController _returnvalue))
    (Default|NotifyMovableForward _asroomba_aicontroller true)))

(event OnComponentEndOverlap(Cylinder)
  (params (OtherActor :type Actor%20Object%20Reference) (OtherComp :type Primitive%20Component%20Object%20Reference) (OtherBodyIndex :type Integer))
  ;[1 1 1] オブジェクトに当たった時の挙動
  (Utilities|FlowControl|DoOnce false) ; enters at Reset
)

(event EventBeginPlay)

(event EventTick
  (params (DeltaSeconds :type Float%20%28single-precision%29))
  (bind _returnvalue (Transformation|GetActorLocation))
  (Collision|LineTraceByChannel _returnvalue (+ _returnvalue (* (Transformation|GetActorForwardVector) (Variables|Default|GetGoForwardSensorLength))) "TraceTypeQuery1" false 0 "ForOneFrame"))

(fn ConstructionScript)