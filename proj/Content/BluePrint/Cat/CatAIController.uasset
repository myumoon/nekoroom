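; AI controller for the cat that supplies its behavior tree with movement and jump targets.
; On BeginPlay it sets up CatBlackboard and stores the first CatMovePoint actor found in the level under the MovePoint key.
; A separate Initialize function writes the supplied JumpPointMesh to the blackboard and then runs CatBehaviourTree, so the tree starts only when that function is called.
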(event EventBeginPlay
  (bind _blackboardcomponent (Class|AIController|UseBlackboard "/Game/BluePrint/Cat/CatBlackboard.CatBlackboard"))
  (bind _outactors (Actor|GetAllActorsOfClass "/Game/BluePrint/Cat/CatMovePoint.CatMovePoint_C"))
  (AI|Components|Blackboard|SetValueasObject _blackboardcomponent (Utilities|Name|MakeLiteralName "MovePoint") (Utilities|Array|Get(acopy) _outactors)))

(event EventTick
  (params (DeltaSeconds :type Float%20%28single-precision%29)))

(fn ConstructionScript)

(fn Initialize
  (params (JumpPointMesh :type Cat%20Jump%20Point%20Mesh%20Object%20Reference))
  (AI|Components|Blackboard|SetValueasObject (AI|GetBlackboard self) (Utilities|Name|MakeLiteralName "JumpPointMesh") JumpPointMesh)
  (AI|RunBehaviorTree "/Game/BluePrint/Cat/CatBehaviourTree.CatBehaviourTree"))