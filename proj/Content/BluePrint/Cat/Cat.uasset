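; Cat character Blueprint that drives its CatAnim animation instance with movement speed and a look-at target.
; BeginPlay initializes CatAnim with the mesh, printing a warning if the cast fails.
; Each Tick passes the velocity length as MoveSpeed and the first ThirdPersonCharacter's location as LookAtPos.
; That character is looked up with GetAllActorsOfClass every frame, and its location is printed for debugging.
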(event EventBeginPlay
  (bind _mesh (Variables|Character|GetMesh))
  (bind _ascat_anim (Utilities|Casting|CastToCatAnim (Components|SkeletalMesh|GetAnimInstance _mesh))
    (:then
      (Default|Initialize _ascat_anim _mesh))
    (:CastFailed
      (Development|PrintText "CatAnim is null"))))

(event Collision|EventActorBeginOverlap
  (params (OtherActor :type Actor%20Object%20Reference)))

(event EventTick
  (params (DeltaSeconds :type Float%20%28single-precision%29))
  (bind _mesh (Variables|Character|GetMesh))
  (bind _returnvalue (Components|SkeletalMesh|GetAnimInstance _mesh))
  (Utilities|IsValid _returnvalue
    (:Is%20Valid
      (bind _ascat_anim (Utilities|Casting|CastToCatAnim _returnvalue))
      (Variables|/Game/BluePrint/Cat/CatAnim.CatAnim_C|SetMoveSpeed _ascat_anim (Math|Vector|VectorLength (Variables|/Script/Engine.MovementComponent|GetVelocity (Variables|Character|GetCharacterMovement))))
      (bind _outactors (Actor|GetAllActorsOfClass "/Game/ThirdPersonBP/Blueprints/ThirdPersonCharacter.ThirdPersonCharacter_C"))
      (Development|PrintString (Utilities|String|ToString(Vector) (Transformation|GetActorLocation (Utilities|Array|Get(acopy) _outactors))))
      (Variables|/Game/BluePrint/Cat/CatAnim.CatAnim_C|SetLookAtPos _ascat_anim (Transformation|GetActorLocation (Utilities|Array|Get(acopy) _outactors))))))

(fn ConstructionScript)