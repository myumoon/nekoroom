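; Behavior tree task that turns the AI-controlled pawn through roughly a half turn in yaw, presumably to the right.
; On execute it resets an accumulated rotation counter.
; Each AI tick it adds a frame-rate-independent yaw step from RotDegPerSecond to the pawn's rotation and the counter, finishing successfully once the total passes 165 degrees.
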(event EventReceiveTickAI
  (params (OwnerController :type AI%20Controller%20Object%20Reference) (ControlledPawn :type Pawn%20Object%20Reference) (DeltaSeconds :type Float%20%28single-precision%29))
  (bind _rotdegpersecond (Variables|Default|GetRotDegPerSecond))
  (bind _returnvalue (* DeltaSeconds _rotdegpersecond))
  (Transformation|SetActorRotation ControlledPawn (Math|Rotator|CombineRotators (Transformation|GetActorRotation ControlledPawn) (Math|Rotator|MakeRotator 0.0 0.0 _returnvalue)))
  (bind _output_get (Variables|Default|SetRotation (+ (Variables|Default|GetRotation) _returnvalue)))
  (if (> _output_get 165.0)
    (AI|BehaviorTree|FinishExecute true)))

(event EventReceiveExecuteAI
  (params (OwnerController :type AI%20Controller%20Object%20Reference) (ControlledPawn :type Pawn%20Object%20Reference))
  (Variables|Default|SetRotation 0.0))