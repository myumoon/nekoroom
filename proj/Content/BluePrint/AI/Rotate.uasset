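; Behavior tree task that turns the AI-controlled pawn in place until it can move forward.
; Each tick adds a frame-rate-independent yaw step, scaled by RotDegPerSecond, to the pawn's rotation.
; It then reads the MovableForward blackboard bool and finishes with success once that is true.
; The task has no failure path of its own, and its End function is an empty stub.
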(event EventReceiveTickAI
  (params (OwnerController :type AI%20Controller%20Object%20Reference) (ControlledPawn :type Pawn%20Object%20Reference) (DeltaSeconds :type Float%20%28single-precision%29))
  (Transformation|SetActorRotation ControlledPawn (Math|Rotator|CombineRotators (Transformation|GetActorRotation ControlledPawn) (Math|Rotator|MakeRotator 0.0 0.0 (* DeltaSeconds (Variables|Default|GetRotDegPerSecond)))))
  (if (ScalableFloat|GetValueasBool (Class|BTFunctionLibrary|GetOwnersBlackboard) (Utilities|Name|MakeLiteralName "MovableForward"))
    (AI|BehaviorTree|FinishExecute true)))

(fn End)