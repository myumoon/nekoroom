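; MoveForward is a Behavior Tree task that pushes the controlled pawn along its forward vector.
; Each tick it adds delta time to a timer capped at AccTime, zeroed only once by a DoOnce, and eases the step in from zero to Speed.
; It sets the location without sweep or delta-time scaling, so Speed is per tick, then finishes as failed after every step.
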(event EventReceiveTickAI
  (params (OwnerController :type AI%20Controller%20Object%20Reference) (ControlledPawn :type Pawn%20Object%20Reference) (DeltaSeconds :type Float%20%28single-precision%29))
  (bind _acctime (Variables|Default|GetAccTime))
  (Utilities|FlowControl|Sequence
    (:then_0
      (Utilities|FlowControl|DoOnce false
        (:Completed
          (Variables|Default|SetCurrentAccTime 0.0))))
    (:then_1
      (bind _output_get (Variables|Default|SetCurrentAccTime (Math|Float|Min(Float) _acctime (+ DeltaSeconds (Variables|Default|GetCurrentAccTime)))))
      (Transformation|SetActorLocation ControlledPawn (+ (* (Transformation|GetActorForwardVector ControlledPawn) (Math|Interpolation|Ease "EaseIn" (/ _output_get _acctime) 0.0 (Variables|Default|GetSpeed) 2.0)) (Transformation|GetActorLocation ControlledPawn)) false false)
      (AI|BehaviorTree|FinishExecute false))))