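; NekoRoomPlayer is the player character that can toggle wall climbing, flagged by an exclamation mark.
; Capsule hits enable climbing and show the mark, and a forward line trace clears both, though IsWall's component-count test (>= 0) always passes.
; Climbing switches to Flying with rotation rate zeroed, while movement input pushes forward into the wall and moves vertically.
; A per-tick face-height sphere trace turns the actor toward "Wall"-tagged hits, with debug output.
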(event OnComponentHit(CapsuleComponent)
  (params (OtherActor :type Actor%20Object%20Reference) (OtherComp :type Primitive%20Component%20Object%20Reference) (NormalImpulse :type Vector :default "0, 0, 0") (Hit :type Hit%20Result%20Structure%20%28by%20ref%29))
  (bind _isobj (CallFunction|IsWall OtherActor))
  (if _isobj
    (CallFunction|SetVisibleExclamation true)
    (Variables|Default|SetClimbable true)))

(event OnComponentBeginOverlap(WallHitSphere)
  (params (OtherActor :type Actor%20Object%20Reference) (OtherComp :type Primitive%20Component%20Object%20Reference) (OtherBodyIndex :type Integer) (bFromSweep :type Boolean) (SweepResult :type Hit%20Result%20Structure%20%28by%20ref%29))
  (Development|PrintString "Hello"))

(event EventBeginPlay
  (Utilities|FlowControl|Sequence
    (:then_0
      (CallFunction|SetVisibleExclamation false))))

(event EventActorBeginOverlap
  (params (OtherActor :type Actor%20Object%20Reference)))

(event EventTick
  (params (DeltaSeconds :type Float%20%28single-precision%29))
  (bind _returnvalue (CallFunction|MakeFaceOffset))
  (bind _capsulecomponent (Variables|Default|GetCapsuleComponent))
  (bind _returnvalue_2 (Transformation|GetWorldLocation _capsulecomponent))
  (bind _returnvalue_3 (+ _returnvalue _returnvalue_2))
  (CallFunction|UpdateEventTick DeltaSeconds (Math|Vector|MakeVector (stale Input|AxisEvents|InputAxisMoveRight AxisValue) 0.0 (stale Input|AxisEvents|InputAxisMoveForward AxisValue)))
  (bind (_outhit _returnvalue_4) (Class|KismetSystemLibrary|SphereTraceSingleNEW _returnvalue_3 (+ _returnvalue_3 (* (Transformation|GetActorForwardVector) 5e+01)) 3e+01 "TraceTypeQuery1" false 0 "ForOneFrame" true))
  (if _returnvalue_4
    ;[1 1 1] todo:なんか柱とのヒットでここがfalseになる
    (Development|PrintString (Utilities|GetDisplayName (.HitActor (Collision|BreakHitResult _outhit))))
    (if (Actor|ActorHasTag (.HitActor (Collision|BreakHitResult _outhit)) "Wall")
      (Utilities|FlowControl|Sequence
        (:then_0
          (Transformation|SetActorRotation (Math|Rotator|MakeRotator (.Roll (Math|Rotator|BreakRotator (Math|Rotator|FindLookatRotation (Transformation|GetActorLocation) (.ImpactPoint (Collision|BreakHitResult _outhit))))) 0.0 (.Yaw (Math|Rotator|BreakRotator (Math|Rotator|FindLookatRotation (Transformation|GetActorLocation) (.ImpactPoint (Collision|BreakHitResult _outhit))))))))
        (:then_1
          (Transformation|SetWorldLocation (Variables|Default|GetSphere) (.ImpactPoint (Collision|BreakHitResult _outhit)) false true))
        (:then_2
          (Development|PrintString "Hello"))))))

(event Input|ActionEvents|InputActionClimb
  (params (Key :type Key%20Structure :default "AnyKey"))
  (:Pressed
    (if (Variables|Default|GetClimbable)
      (CallFunction|ToggleClimb))))

(event Input|AxisEvents|InputAxisMoveForward
  (params (AxisValue :type Float%20%28single-precision%29)))

(event Input|AxisEvents|InputAxisMoveRight
  (params (AxisValue :type Float%20%28single-precision%29)))

(fn ConstructionScript
  (|CallParentFunction))

(fn SetVisibleExclamation
  (params (visible :type Boolean))
  (Rendering|SetVisibility (Variables|Default|GetExclamation) visible true))

(fn CheckClimbableWall)

(fn UpdateEventTick
  (params (delta :type Float%20%28single-precision%29) (InputMove :type Vector))
  (bind _returnvalue (Transformation|GetActorLocation))
  (Utilities|FlowControl|Sequence
    (:then_0
      ;[1 1 1] ビックリマーク削除判定
      (if (Variables|Default|GetClimbable)
        (bind (_outhit _returnvalue_2) (Collision|LineTraceByChannel _returnvalue (+ _returnvalue (* (Transformation|GetActorForwardVector) (LocalVariables|GetClimbableWallDistance))) "TraceTypeQuery1" false 0 "None"))
        (bind _isobj (CallFunction|IsWall (.HitActor (Collision|BreakHitResult _outhit))))
        (if (or (not _isobj) (not _returnvalue_2))
          (Variables|Default|SetClimbable false)
          (CallFunction|SetVisibleExclamation false)
          (return))))
    (:then_1
      ;[1 1 1] 常に前方向の入力を与えて壁に吸い付かせる
      (if (Variables|Default|GetClimbing)
        (if (> (Math|Vector|VectorLengthSquared InputMove) 0.0)
          (Class|PawnMovementComponent|AddInputVector (Variables|Character|GetCharacterMovement) (* (Transformation|GetActorForwardVector) 5.0) true)
          ;[1 1 1] 上下移動
          (Class|PawnMovementComponent|AddInputVector (Variables|Character|GetCharacterMovement) (* (* (Transformation|GetActorUpVector) (.Z (Math|Vector|BreakVector InputMove))) 5.0) false))))))

(fn IsWall
  (params (obj :type Actor%20Object%20Reference))
  (return (>= (Utilities|Array|Length (Actor|GetComponentsByClass obj "/Script/Engine.InstancedStaticMeshComponent")) 0)))

(fn Climb
  (params (climbWall :type Boolean))
  (bind _charactermovement (Variables|Character|GetCharacterMovement))
  (bind _charactermovement_2 (Variables|Character|GetCharacterMovement))
  (Physics|SetEnableGravity (Variables|Default|GetCapsuleComponent) climbWall)
  (if climbWall
    (Variables|/Script/Engine.MovementComponent|SetVelocity (Variables|Character|GetCharacterMovement) "0, 0, 0")
    (Pawn|Components|CharacterMovement|SetMovementMode _charactermovement "MOVE_Flying" 0)
    (Variables|Default|SetPrevRotationRate (Variables|/Script/Engine.CharacterMovementComponent|GetRotationRate _charactermovement))
    (Variables|/Script/Engine.CharacterMovementComponent|SetRotationRate _charactermovement_2 "0, 0, 0")
    (else
      (Pawn|Components|CharacterMovement|SetMovementMode _charactermovement "MOVE_Walking" 0)
      (Variables|/Script/Engine.CharacterMovementComponent|SetRotationRate _charactermovement_2 (Variables|Default|GetPrevRotationRate)))))

(fn ToggleClimb
  (bind _output_get (Variables|Default|SetClimbing (not (Variables|Default|GetClimbing))))
  (CallFunction|Climb _output_get))

(fn IsClimbing
  (return (Variables|Default|GetClimbing)))

(fn MakeFaceOffset
  (bind _capsulecomponent (Variables|Default|GetCapsuleComponent))
  (return (Math|Vector|MakeVector 0.0 0.0 (- (Components|Capsule|GetScaledCapsuleHalfHeight _capsulecomponent) (Components|Capsule|GetScaledCapsuleRadius _capsulecomponent)))))